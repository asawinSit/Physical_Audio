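; Test actor that plays an impact sound scaled by speed when it hits something, with debug output.
; On Hit, it draws a long-lived debug circle at the impact point and plays a MetaSound at the actor's location.
; The hit component's velocity magnitude is remapped, with clamping, to set the sound's volume.
; Tick prints the Cube component's current speed to help observe the values.
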(event EventBeginPlay)

(event Collision|EventActorBeginOverlap
  (params (OtherActor :type Actor%20Object%20Reference)))

(event EventTick
  (params (DeltaSeconds :type Float%20%28single-precision%29))
  (Development|PrintString (Utilities|String|ToString(Float) (Math|Vector|VectorLength (Transformation|GetComponentVelocity (Variables|Default|GetCube))))))

(event Collision|EventHit
  (params (MyComp :type Primitive%20Component%20Object%20Reference) (Other :type Actor%20Object%20Reference) (OtherComp :type Primitive%20Component%20Object%20Reference) (bSelfMoved :type Boolean) (HitLocation :type Vector :default "0, 0, 0") (HitNormal :type Vector :default "0, 0, 0") (NormalImpulse :type Vector :default "0, 0, 0") (Hit :type Hit%20Result%20Structure%20%28by%20ref%29))
  (Rendering|Debug|DrawDebugCircle (.impactpoint Hit) 1e+01 12 "(R=0.012100,G=0.000000,B=1.000000,A=1.000000)" 1e+02 0.0 "0.000000,1.000000,0.000000" "0.000000,0.000000,1.000000")
  (Audio|PlaySoundatLocation "/Game/NewMetaSoundSource.NewMetaSoundSource" (Transformation|GetActorLocation) "0, 0, 0" (Math|Float|MapRangeClamped (Math|Vector|VectorLength (Transformation|GetComponentVelocity MyComp)) 2e+02 6e+02 0.1 2.0) 1.0 0.0 0 0 0 0))

(fn ConstructionScript)